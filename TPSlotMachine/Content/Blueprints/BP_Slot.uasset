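; BP_Slot is a slot machine actor with a lever and three reels, spun when the actor is hit.
; A hit while the lever is at rest tilts it and snaps each reel to a random one of sixteen positions, staggered by short delays.
; Tick eases the lever back at a constant rate, blocking new spins until it returns.
; Only the first two reel results are compared, and a match prints a message.
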(event EventBeginPlay)

(event Collision|EventActorBeginOverlap
  (params (OtherActor :type Actor%20Object%20Reference)))

(event EventTick
  (params (DeltaSeconds :type Float%20%28single-precision%29))
  (bind _output_get (Variables|Default|SetLever%20Angle (Math|Float|Max(Float) (- (Variables|Default|GetLever%20Angle) (* DeltaSeconds 1e+01)) 0.0)))
  (Transformation|SetRelativeRotation (Variables|Default|GetLever) (Math|Rotator|MakeRotator _output_get 0.0 0.0) false false))

(event Collision|EventHit
  (params (MyComp :type Primitive%20Component%20Object%20Reference) (Other :type Actor%20Object%20Reference) (OtherComp :type Primitive%20Component%20Object%20Reference) (bSelfMoved :type Boolean) (HitLocation :type Vector :default "0, 0, 0") (HitNormal :type Vector :default "0, 0, 0") (NormalImpulse :type Vector :default "0, 0, 0") (Hit :type Hit%20Result%20Structure%20%28by%20ref%29))
  (if (== (Variables|Default|GetLever%20Angle) 0.0)
    (bind _output_get (Variables|Default|SetLever%20Angle 45.0))
    (Transformation|SetRelativeRotation (Variables|Default|GetLever) (Math|Rotator|MakeRotator _output_get 0.0 0.0) false false)
    (bind _reelindex (CallFunction|Spin (Variables|Default|GetCylinder1)))
    (Utilities|FlowControl|Delay 0.2)
    (bind _reelindex_2 (CallFunction|Spin (Variables|Default|GetCylinder2)))
    (Utilities|FlowControl|Delay 0.2)
    (CallFunction|Spin (Variables|Default|GetCylinder3))
    (if (== _reelindex _reelindex_2)
      (Development|PrintString "Hello" true true "(R=0.000000,G=0.660000,B=1.000000,A=1.000000)" 1e+01))))

(fn ConstructionScript)

(fn Spin
  (params (Reel :type Static%20Mesh%20Component%20Object%20Reference))
  (bind _output_get (LocalVariables|SetResult (Math|Random|RandomIntegerinRange 0 15)))
  (Transformation|SetRelativeRotation Reel (Math|Rotator|MakeRotator 9e+01 (* _output_get (Math|Float|MakeLiteralFloat 22.5)) 9e+01) false false)
  (return (LocalVariables|GetResult)))